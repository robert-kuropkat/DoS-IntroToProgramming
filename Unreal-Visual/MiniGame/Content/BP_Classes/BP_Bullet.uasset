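; BP_Bullet is a projectile actor that plays a shooting sound when spawned and flies toward negative Y.
; Tick moves it with a swept world offset scaled by Speed and delta time, then destroys it once its Y drops to the YDestroyAt off-screen threshold.
; BeginPlay also sets a unit scale before and after a short delay, so the size stays the same.
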(event `self.ReceiveBeginPlay`
  (`GameplayStatics.PlaySound2D` "/Game/Audio/sfx_shoot.sfx_shoot" 1.0 1.0 0.0 null null)
  (`self.SetActorRelativeScale3D` (1.0 1.0 1.0))
  (`KismetSystemLibrary.Delay` 0.2)
  (`self.SetActorRelativeScale3D` (1.0 1.0 1.0)))

(event `self.ReceiveTick`
  (params (DeltaSeconds :type "Float (single-precision)"))
  ; Move Bullet Up
  (`self.K2_AddActorWorldOffset` (`KismetMathLibrary.MakeVector` 0.0 (* (`self.Speed`) (`GameplayStatics.GetWorldDeltaSeconds`) -1.0)) true)
  ; If Bullet Off-Screen: Destroy Itself
  (if (<= (.y (`self.K2_GetActorLocation`)) (`self.YDestroyAt`))
    (`self.K2_DestroyActor`)))

(fn `UserConstructionScript`)