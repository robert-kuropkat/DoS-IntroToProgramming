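; Player actor for a flat, screen-bounded shooter, moved in four directions and firing BP_Bullet through Enhanced Input.
; Each move action offsets the actor by speed and delta time, then shares a screen clamp and throttled blip sound.
; Move starts set a direction-specific material and IsMoving, which Tick uses to blink visibility or restore blue when idle.
; The fire cooldown only counts down on each press, not over time.
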(event `self.ReceiveBeginPlay`
  ; EVENT BEGIN PLAY:  Setup Input System
  (`EnhancedInputSubsystemInterface.AddMappingContext` (pcsubsystem `EnhancedInputLocalPlayerSubsystem` (`GameplayStatics.GetPlayerController` 0)) "/Game/InputActions/IMC_Default.IMC_Default" 0 (struct)))

(event `self.ReceiveTick`
  (params (DeltaSeconds :type "Float (single-precision)"))
  ; EVENT TICK:
  ;; If Player Moving
  (if (== (`self.IsMoving`) true)
    ;;; Is Moving True (animate)
    (bind _output_get (set `self.BlinkTimer` (+ (`self.BlinkTimer`) (`GameplayStatics.GetWorldDeltaSeconds`))))
    (if (>= _output_get 0.1)
      (`self.SetActorHiddenInGame` (stale _output_get_2))
      (set `self.BlinkTimer` 0.0)
      (bind _output_get_2 (set `self.Blink` (not (`self.Blink`)))))
    (else
      ;;; Is Moving False (idle)
      (`PrimitiveComponent.SetMaterial` (`self.StaticMeshComponent`) 0 "/Game/Materials/M_Player_Blue.M_Player_Blue")
      (`self.SetActorHiddenInGame` false))))

(event `EnhancedInput|/Game/InputActions/IA_Fire`
  (params (ActionValue :type Boolean) (ElapsedSeconds :type "Float (double-precision)") (TriggeredSeconds :type "Float (double-precision)") (InputAction :type "InputAction Object Reference" :default "/Game/InputActions/IA_Fire.IA_Fire"))
  ; Fire Control
  (:`Started`
    ;; Firing Cool Down
    (bind _output_get (set `self.FireCoolDown` (- (`self.FireCoolDown`) (`GameplayStatics.GetWorldDeltaSeconds`))))
    (if (<= _output_get 0.0)
      (set `self.FireCoolDown` 0.1)
      (`|SpawnActorFromClass` "/Game/BP_Classes/BP_Bullet.BP_Bullet_C" (`KismetMathLibrary.Conv_VectorToTransform` (`KismetMathLibrary.MakeVector` (.x (.location (`self.GetTransform`))) (- (.y (.location (`self.GetTransform`))) (`self.BulletInitialOffset`)))) "Undefined" "MultiplyWithRoot" null null))))

(event `EnhancedInput|/Game/InputActions/IA_MoveDown`
  (params (ActionValue :type Boolean) (ElapsedSeconds :type "Float (double-precision)") (TriggeredSeconds :type "Float (double-precision)") (InputAction :type "InputAction Object Reference" :default "/Game/InputActions/IA_MoveDown.IA_MoveDown"))
  ; Player Movement Control
  ;; Player Move Down Control
  (:`Triggered`
    (`self.K2_AddActorWorldOffset` (`KismetMathLibrary.MakeVector` 0.0 (* (`GameplayStatics.GetWorldDeltaSeconds`) (`self.PlayerSpeed`))))
    ;; Player Movement Sound FX
    (`self.K2_SetActorLocation` (`KismetMathLibrary.MakeVector` (`KismetMathLibrary.FClamp` (.x (`self.K2_GetActorLocation`)) -950.0 950.0) (`KismetMathLibrary.FClamp` (.y (`self.K2_GetActorLocation`)) -500.0 500.0)) :!label _label)
    (bind _output_get (set `self.SoundCoolDown` (- (`self.SoundCoolDown`) (`GameplayStatics.GetWorldDeltaSeconds`))))
    (if (<= _output_get 0.0)
      (`GameplayStatics.PlaySound2D` "/Game/Audio/sfx_blip.sfx_blip" 1.0 1.0 0.0 null null)
      (set `self.SoundCoolDown` 0.15)))
  (:`Started`
    (`PrimitiveComponent.SetMaterial` (`self.StaticMeshComponent`) 0 "/Game/Materials/M_Player_Orange.M_Player_Orange")
    (set `self.IsMoving` true))
  (:`Completed`
    (set `self.IsMoving` false)))

(event `EnhancedInput|/Game/InputActions/IA_MoveRight`
  (params (ActionValue :type Boolean) (ElapsedSeconds :type "Float (double-precision)") (TriggeredSeconds :type "Float (double-precision)") (InputAction :type "InputAction Object Reference" :default "/Game/InputActions/IA_MoveRight.IA_MoveRight"))
  ; Player Movement Control
  ;; Player Move Right Control
  (:`Triggered`
    (`self.K2_AddActorWorldOffset` (`KismetMathLibrary.MakeVector` (* (`GameplayStatics.GetWorldDeltaSeconds`) (`self.PlayerSpeed`))))
    (goto _label))
  (:`Started`
    (`PrimitiveComponent.SetMaterial` (`self.StaticMeshComponent`) 0 "/Game/Materials/M_Player_Yellow.M_Player_Yellow")
    (set `self.IsMoving` true))
  (:`Completed`
    (set `self.IsMoving` false)))

(event `EnhancedInput|/Game/InputActions/IA_MoveLeft`
  (params (ActionValue :type Boolean) (ElapsedSeconds :type "Float (double-precision)") (TriggeredSeconds :type "Float (double-precision)") (InputAction :type "InputAction Object Reference" :default "/Game/InputActions/IA_MoveLeft.IA_MoveLeft"))
  ; Player Movement Control
  ;; Player Mov Left Control
  (:`Triggered`
    (`self.K2_AddActorWorldOffset` (`KismetMathLibrary.MakeVector` (* (* (`GameplayStatics.GetWorldDeltaSeconds`) (`self.PlayerSpeed`)) -1.0)))
    (goto _label))
  (:`Started`
    (`PrimitiveComponent.SetMaterial` (`self.StaticMeshComponent`) 0 "/Game/Materials/M_Player_Green.M_Player_Green")
    (set `self.IsMoving` true))
  (:`Completed`
    (set `self.IsMoving` false)))

(event `EnhancedInput|/Game/InputActions/IA_MoveUp`
  (params (ActionValue :type Boolean) (ElapsedSeconds :type "Float (double-precision)") (TriggeredSeconds :type "Float (double-precision)") (InputAction :type "InputAction Object Reference" :default "/Game/InputActions/IA_MoveUp.IA_MoveUp"))
  ; Player Movement Control
  ;; Player Move Up Control
  (:`Triggered`
    (`self.K2_AddActorWorldOffset` (`KismetMathLibrary.MakeVector` 0.0 (* (* (`GameplayStatics.GetWorldDeltaSeconds`) (`self.PlayerSpeed`)) -1.0)))
    (goto _label))
  (:`Started`
    (`PrimitiveComponent.SetMaterial` (`self.StaticMeshComponent`) 0 "/Game/Materials/M_Player_Red.M_Player_Red")
    (set `self.IsMoving` true))
  (:`Completed`
    (set `self.IsMoving` false)))

(fn `UserConstructionScript`)